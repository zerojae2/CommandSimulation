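; BP_Test drives minimap icons that mirror the positions of the BP_Robot1 actors in the level.
; On BeginPlay it spawns an icon actor per robot at its X/Y scaled down by a constant divisor, at a fixed height.
; A self-calling delayed event repeatedly moves each icon to its index-matched robot's scaled position, re-triggering from inside the nested loop unless Reset is set.
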(event Custom|spawn%20minimap%20icon
  (bind _outactors (Actor|GetAllActorsOfClass "/Game/BP_Robot1.BP_Robot1_C"))
  (bind _output_get (Variables|Default|SetRobot%20array _outactors))
  (for _array_element _output_get
    (bind _returnvalue (Game|SpawnActorfromClass "/Game/BP_MinimapRobotIcon.BP_MinimapRobotIcon_C" (Math|Transform|MakeTransform (Math|Vector|MakeVector (/ (.x (.location (Transformation|GetActorTransform _array_element))) 65.0) (/ (.y (.location (Transformation|GetActorTransform _array_element))) 65.0) 1.51e+03) "0, 0, 0" "1.000000,1.000000,1.000000") "Undefined" "MultiplyWithRoot" 0 0))
    (Utilities|Array|Add (Variables|Default|GetMini%20map%20Robot%20array) _returnvalue)))

(event Custom|get%20coordinate
  (Utilities|FlowControl|Delay 0.2)
  (for (_array_element _array_index) (Variables|Default|GetRobot%20array)
    (for (_array_element_2 _array_index_2) (Variables|Default|GetMini%20map%20Robot%20array)
      (if (== _array_index _array_index_2)
        (Transformation|SetActorLocation _array_element_2 (Math|Vector|MakeVector (/ (.x (.location (Transformation|GetActorTransform _array_element))) 65.0) (/ (.y (.location (Transformation|GetActorTransform _array_element))) 65.0) 1.51e+03) false false)
        (if (not (== (Variables|Default|Getreset) 1))
          (CallFunction|GetCoordinate))))))

(event EventBeginPlay
  (CallFunction|SpawnMinimapIcon)
  (CallFunction|GetCoordinate))

(fn ConstructionScript)