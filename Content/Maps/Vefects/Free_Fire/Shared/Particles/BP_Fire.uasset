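; BP_Fire is a fire actor that seeds BP_FireCheck actors around itself, apparently to propagate fire.
; On BeginPlay it waits DuplicateInterval, then spawns one checker per DirectionVector entry, offset from its location by DuplicateDistance along the normalized direction.
; The spawn pass runs once per instance, with no checks in this graph; the Hit event and construction script are empty.
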(event Collision|EventHit
  (params (MyComp :type Primitive%20Component%20Object%20Reference) (Other :type Actor%20Object%20Reference) (OtherComp :type Primitive%20Component%20Object%20Reference) (bSelfMoved :type Boolean) (HitLocation :type Vector :default "0, 0, 0") (HitNormal :type Vector :default "0, 0, 0") (NormalImpulse :type Vector :default "0, 0, 0") (Hit :type Hit%20Result%20Structure%20%28by%20ref%29)))

(event EventBeginPlay
  (Utilities|FlowControl|Delay (Variables|Default|GetDuplicateInterval))
  (for _array_element (Variables|Default|GetDirectionVector)
    (Game|SpawnActorfromClass "/Game/Vefects/Free_Fire/Blueprints/BP_FireCheck.BP_FireCheck_C" (Math|Conversions|ToTransform(Vector) (+ (* (Math|Vector|Normalize _array_element) (Variables|Default|GetDuplicateDistance)) (Transformation|GetActorLocation))) "Undefined" "MultiplyWithRoot" 0 0)))

(fn ConstructionScript)