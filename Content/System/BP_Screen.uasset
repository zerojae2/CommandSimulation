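; BP_Screen is an in-game screen that shows the camera material matching the selected robot.
; On BeginPlay it caches all BP_Robot1 actors, then runs a self-repeating polling event every 0.2 seconds.
; For each robot flagged IsSelected, it applies the material at the same index in CamMaterial to the Screen and clears the flag, printing debug text for each check.
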(event Custom|change%20cam
  (for (_array_element _array_index) (Variables|Default|Getrobot)
    (Variables|Default|Setselected%20robot%20index _array_index)
    (bind _output_get (Variables|Default|Setselected%20robot _array_element))
    (if (Variables|/Game/System/BP_Robot1.BP_Robot1_C|GetIsSelected _output_get)
      (Development|PrintString "TRUE")
      (Rendering|Material|SetMaterial (Variables|Default|GetScreen) 0 (Utilities|Array|Get(acopy) (Variables|Default|Getcam_material) (Variables|Default|Getselected%20robot%20index)))
      (Variables|/Game/System/BP_Robot1.BP_Robot1_C|SetIsSelected (Variables|Default|Getselected%20robot) false)
      (else
        (Development|PrintString "FASLE"))))
  (Utilities|FlowControl|Delay 0.2)
  (CallFunction|ChangeCam))

(event EventBeginPlay
  (bind _outactors (Actor|GetAllActorsOfClass "/Game/System/BP_Robot1.BP_Robot1_C"))
  (Variables|Default|Setrobot _outactors)
  (CallFunction|ChangeCam))

(fn ConstructionScript)